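; BP_Monster1 is an AI monster that uses zombie animations and damages actors of class Zombie.
; Custom events, with no callers in this graph, play looping walk, one-shot attack and death animations directly on the Mesh.
; The attack event briefly enables Capsule overlap events after a delay, so overlaps in that window apply damage.
; SCDelay serves as the death event, destroying the actor after a delay.
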(event OnComponentBeginOverlap(Capsule)
  (params (OverlappedComponent :type Primitive%20Component%20Object%20Reference) (OtherActor :type Actor%20Object%20Reference) (OtherComp :type Primitive%20Component%20Object%20Reference) (OtherBodyIndex :type Integer) (bFromSweep :type Boolean) (SweepResult :type Hit%20Result%20Structure%20%28by%20ref%29))
  (bind _aszombie (Utilities|Casting|CastToZombie OtherActor))
  (Game|Damage|ApplyDamage _aszombie 0.2 0 self))

(event EventBeginPlay
  (|CallParentFunction) ; This node is disabled and will not be called.\nDrag off pins to build functionality.
)

(event Collision|EventActorBeginOverlap
  (params (OtherActor :type Actor%20Object%20Reference)))

(event EventTick
  (params (DeltaSeconds :type Float%20%28single-precision%29))
  (|CallParentFunction DeltaSeconds) ; This node is disabled and will not be called.\nDrag off pins to build functionality.
)

(event EventSCWalkAnim
  (Components|Animation|PlayAnimation (Variables|Character|GetMesh) "/Game/MonsterAssets/Monster1/Zombie_Walk1.Zombie_Walk1" true))

(event EventSCAttackAnim
  (bind _capsule (Variables|Default|GetCapsule))
  (Utilities|FlowControl|Delay 0.5)
  (Variables|/Script/Engine.PrimitiveComponent|SetbGenerateOverlapEvents _capsule true)
  (Components|Animation|PlayAnimation (Variables|Character|GetMesh) "/Game/MonsterAssets/Monster1/Zombie_Attack1.Zombie_Attack1" false)
  (Utilities|FlowControl|Delay 2.0)
  (Variables|/Script/Engine.PrimitiveComponent|SetbGenerateOverlapEvents _capsule false))

(event EventSCDelay
  (Components|Animation|PlayAnimation (Variables|Character|GetMesh) "/Game/MonsterAssets/Monster1/Zombie_Death1.Zombie_Death1" false)
  (Utilities|FlowControl|Delay 3.0)
  (Actor|DestroyActor))

(fn ConstructionScript
  (|CallParentFunction))