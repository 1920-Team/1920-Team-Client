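; BP_NPC1 is a zombie NPC that chases seen pawns, plays an attack animation and dies from damage.
; PawnSensing triggers AI MoveTo on the seen pawn, playing the attack on arrival without applying damage.
; Each hit subtracts fixed health; at zero it destroys itself and decrements BP_NPCSpawner's count.
; All logic runs on authority, including an NPC_UI widget projected each Tick from the "HP Socket" to player 0's screen.
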(event OnSeePawn(PawnSensing)
  (params (Pawn :type Pawn%20Object%20Reference))
  (Networking|SwitchHasAuthority
    (:Authority
      (CallFunction|FollowPlayer))))

(event Custom|FollowPlayer
  (Networking|SwitchHasAuthority
    (:Authority
      (AI|AIMoveTo self "0, 0, 0" (stale OnSeePawn(PawnSensing) Pawn) 5.0 false
        (:OnSuccess
          (Development|PrintText "Attack")
          (Components|Animation|PlayAnimation (Variables|Character|GetMesh) "/Game/MonsterAssets/Monster2/Zombie_Attack2.Zombie_Attack2" false))))))

(event EventBeginPlay
  (Networking|SwitchHasAuthority
    (:Authority
      (bind _returnvalue (UserInterface|CreateWidget "/Game/BluePrints/UI/NPC_UI.NPC_UI_C" 0 self))
      (bind _output_get (Variables|Default|SetNPC_UI _returnvalue))
      (UserInterface|Viewport|AddtoViewport _output_get 0))))

(event Game|Damage|EventAnyDamage
  (params (Damage :type Float%20%28single-precision%29) (DamageType :type Damage%20Type%20Object%20Reference) (InstigatedBy :type Controller%20Object%20Reference) (DamageCauser :type Actor%20Object%20Reference))
  (Networking|SwitchHasAuthority
    (:Authority
      (bind _output_get (Variables|Default|SetHealth (- (Variables|Default|GetHealth) 0.35)))
      (if (<= _output_get 0.0)
        (Actor|DestroyActor)
        (bind _returnvalue (Actor|GetActorOfClass "/Game/BluePrints/AI/BP_NPCSpawner.BP_NPCSpawner_C"))
        (Math|Integer|DecrementInt (Variables|/Game/BluePrints/AI/BP_NPCSpawner.BP_NPCSpawner_C|GetNPCCount _returnvalue))))))

(event EventEndPlay
  (params (EndPlayReason :type EEndPlayReason%20Enum :default "Destroyed"))
  (Networking|SwitchHasAuthority
    (:Authority
      (Widget|RemovefromParent (Variables|Default|GetNPC_UI)))))

(event EventTick
  (params (DeltaSeconds :type Float%20%28single-precision%29))
  (Networking|SwitchHasAuthority
    (:Authority
      (Class|UserWidget|SetPositioninViewport (Variables|Default|GetNPC_UI) (.ScreenLocation (Class|PlayerController|ProjectWorldLocationtoScreen (Game|GetPlayerController 0) (Transformation|GetSocketLocation (Variables|Character|GetMesh) "HP Socket") false)) true))))

(fn ConstructionScript)