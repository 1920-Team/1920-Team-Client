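; Networked zombie NPC that chases pawns it senses, attacks up close and shows a screen-projected health widget above its socket.
; On the server, pawn sensing drives AIMoveTo, or a DoOnce-gated attack pause when Tick's XY distance to the first Zombie-class actor is short.
; CS/SC event pairs relay widget and damage handling.
; Each hit subtracts fixed health; death broadcasts MiniMonsterKilled and decrements BP_NPCSpawner's count.
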(event OnSeePawn(PawnSensing)
  (params (Pawn :type Pawn%20Object%20Reference))
  (Networking|SwitchHasAuthority
    (:Authority
      (CallFunction|FollowPlayer))))

(event Custom|FollowPlayer
  (Networking|SwitchHasAuthority
    (:Authority
      (if (< (Variables|Default|GetDistance) 3e+02)
        (Development|PrintText "Attack")
        (Utilities|FlowControl|DoOnce false :!label _label
          (:Completed
            (CallFunction|SCAttackAnim)
            (Variables|/Script/Engine.CharacterMovementComponent|SetMaxWalkSpeed (Variables|Character|GetCharacterMovement) 0.0)
            (Utilities|FlowControl|Delay 2.5)
            (Variables|/Script/Engine.CharacterMovementComponent|SetMaxWalkSpeed (Variables|Character|GetCharacterMovement) 1e+02)
            (CallFunction|SCWalkAnim)
            (goto _label Reset)))
        (else
          (AI|AIMoveTo self "0, 0, 0" (stale OnSeePawn(PawnSensing) Pawn) 5.0 false
            (:OnSuccess
              (Development|PrintText "Move"))))))))

(event Custom|SC_AddViewportWidget
  (CallFunction|CreateWidget)
  (CallFunction|AddViewportWidget))

(event Custom|CS_DamageProcess
  (CallFunction|DamageProcess)
  (CallFunction|SCDamageProcess))

(event Custom|CS_AddViewportWidget
  (CallFunction|SCAddViewportWidget))

(event Custom|SC_DamageProcess
  ;[1 1 1] Call Update HP
)

(event Custom|CS_DestroyWidget
  (CallFunction|SCDestroyWidget))

(event Custom|SC_DestroyWidget
  (CallFunction|DestroyWidget))

(event Custom|SC_AttackAnim
  (Components|Animation|PlayAnimation (Variables|Character|GetMesh) "/Game/MonsterAssets/Monster1/Zombie_Attack1.Zombie_Attack1" false))

(event Custom|SC_WalkAnim
  (Components|Animation|PlayAnimation (Variables|Character|GetMesh) "/Game/MonsterAssets/Monster1/Zombie_Walk1.Zombie_Walk1" true))

(event Custom|Delay
  (Utilities|FlowControl|Delay 3.0))

(event EventBeginPlay
  (CallFunction|CSAddViewportWidget))

(event Game|Damage|EventAnyDamage
  (params (Damage :type Float%20%28single-precision%29) (DamageType :type Damage%20Type%20Object%20Reference) (InstigatedBy :type Controller%20Object%20Reference) (DamageCauser :type Actor%20Object%20Reference))
  (CallFunction|CSDamageProcess))

(event EventEndPlay
  (params (EndPlayReason :type EEndPlayReason%20Enum :default "Destroyed"))
  (CallFunction|CSDestroyWidget))

(event EventTick
  (params (DeltaSeconds :type Float%20%28single-precision%29))
  (CallFunction|UpdateWidget)
  (bind _returnvalue (Actor|GetActorOfClass "/Game/BluePrints/Zombie/Zombie.Zombie_C"))
  (Variables|Default|SetDistance (Math|Vector|VectorLengthXY (- (Transformation|GetActorLocation _returnvalue) (Transformation|GetActorLocation)))))

(fn ConstructionScript)

(fn DamageProcess
  (bind _output_get (Variables|Default|SetHealth (- (Variables|Default|GetHealth) 0.35)))
  (if (<= _output_get 0.0)
    (Default|CallOnMiniMonsterKilled?)
    (Actor|DestroyActor)
    (bind _returnvalue (Actor|GetActorOfClass "/Game/BluePrints/AI/BP_NPCSpawner.BP_NPCSpawner_C"))
    (Math|Integer|DecrementInt (Variables|/Game/BluePrints/AI/BP_NPCSpawner.BP_NPCSpawner_C|GetNPCCount _returnvalue))))

(fn CreateWidget
  (bind _returnvalue (UserInterface|CreateWidget "/Game/BluePrints/UI/NPC_UI.NPC_UI_C" 0 self))
  (Variables|Default|SetNPC_UI _returnvalue))

(fn UpdateWidget
  (Class|UserWidget|SetPositioninViewport (Variables|Default|GetNPC_UI) (.ScreenLocation (Class|PlayerController|ProjectWorldLocationtoScreen (Game|GetPlayerController 0) (Transformation|GetSocketLocation (Variables|Character|GetMesh) "HP Socket") false)) true))

(fn DestroyWidget
  (Widget|RemovefromParent (Variables|Default|GetNPC_UI)))

(fn AddViewportWidget
  (UserInterface|Viewport|AddtoViewport (Variables|Default|GetNPC_UI) 0))