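; Networked zombie boss for a wave game that becomes damageable once WaveGameState signals all enemies are killed.
; On the server, PawnSensing triggers AIMoveTo or a headbutt that pauses movement, based on Tick's nearest Zombie-class distance.
; Damage scaled by HealthRatio lowers health; death decrements the wave boss count, plays an animation and destroys the actor.
; CS/SC event pairs relay animations and a health-socket-tracking viewport widget.
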(event OnSeePawn(PawnSensing)
  (params (Pawn :type Pawn%20Object%20Reference))
  (Networking|SwitchHasAuthority
    (:Authority
      (CallFunction|FollowPlayer))))

(event Custom|FollowPlayer
  (Networking|SwitchHasAuthority
    (:Authority
      (if (< (Variables|Default|GetDistance) 3e+02)
        (Development|PrintText "Attack")
        (Utilities|FlowControl|DoOnce false :!label _label
          (:Completed
            (if (not (Variables|Default|GetIs%20Dying?))
              (CallFunction|SCAttackAnim)
              (Utilities|AttackTime
                (:Out
                  (CallFunction|SCWalkAnim)
                  (goto _label Reset))))))
        (else
          (AI|AIMoveTo self "0, 0, 0" (stale OnSeePawn(PawnSensing) Pawn) 5.0 false
            (:OnSuccess
              (Development|PrintText "Move"))))))))

(event Custom|SC_DeadAnimation
  (Components|Animation|PlayAnimation (Variables|Character|GetMesh) "/Game/MonsterAssets/Boss/Zombie_Death_Boss.Zombie_Death_Boss" false)
  (Utilities|FlowControl|Delay 3.0)
  (Actor|DestroyActor))

(event Custom|SC_AttackAnim
  (Components|Animation|PlayAnimation (Variables|Character|GetMesh) "/Game/MonsterAssets/Boss/Zombie_Headbutt.Zombie_Headbutt" false))

(event Custom|SC_WalkAnim
  (Components|Animation|PlayAnimation (Variables|Character|GetMesh) "/Game/MonsterAssets/Boss/Zombie_Run.Zombie_Run" true))

(event Custom|ImmunityOff
  (Variables|Default|SetCan%20Take%20Damage? true))

(event Custom|CS_AddViewportWidget
  (CallFunction|SCAddViewportWidget))

(event Custom|SC_addViewportWidget
  (CallFunction|CreateWidgetandAddViewport)
  (CallFunction|UpdateWidget))

(event Custom|CS_DestroyWidget
  (CallFunction|SCDestroyWidget))

(event Custom|SC_DestroyWidget
  (CallFunction|DestroyWidget))

(event Custom|CS_DamageProcess
  (params (Damage :type Float%20%28double-precision%29))
  (Utilities|DamageProcess Damage
    (:Out
      (CallFunction|SCDamageProcess))))

(event Custom|SC_DamageProcess)

(event Custom|CS_Update
  (CallFunction|CalculatetoClosePlayer)
  (CallFunction|SCUpdate))

(event Custom|SC_Update
  (CallFunction|UpdateWidget))

(event EventBeginPlay
  (CallFunction|CSAddViewportWidget)
  (if (Networking|IsServer)
    (bind _aswave_game_state (Utilities|Casting|CastToWaveGameState (Game|GetGameState)))
    (EventDispatchers|BindEventtoAllEnemyKilled _aswave_game_state (delegate Custom|ImmunityOff))))

(event Game|Damage|EventAnyDamage
  (params (Damage :type Float%20%28single-precision%29) (DamageType :type Damage%20Type%20Object%20Reference) (InstigatedBy :type Controller%20Object%20Reference) (DamageCauser :type Actor%20Object%20Reference))
  (if (Networking|IsServer)
    (CallFunction|CSDamageProcess Damage)))

(event EventEndPlay
  (params (EndPlayReason :type EEndPlayReason%20Enum :default "Destroyed")))

(event EventTick
  (params (DeltaSeconds :type Float%20%28single-precision%29))
  (CallFunction|CSUpdate))

(fn ConstructionScript)

(fn CreateWidgetandAddViewport
  (bind _returnvalue (UserInterface|CreateWidget "/Game/BluePrints/UI/NPC_UI3.NPC_UI3_C" 0 self))
  (bind _output_get (Variables|Default|SetNPC_UI _returnvalue))
  (UserInterface|Viewport|AddtoViewport _output_get 0))

(fn DestroyWidget
  (Widget|RemovefromParent (Variables|Default|GetNPC_UI)))

(fn UpdateWidget
  (Class|UserWidget|SetPositioninViewport (Variables|Default|GetNPC_UI) (.ScreenLocation (Class|PlayerController|ProjectWorldLocationtoScreen (Game|GetPlayerController 0) (Transformation|GetSocketLocation (Variables|Character|GetMesh) "HP Socket") false)) true))

(fn CalculatetoClosePlayer
  ;[1 1 1] Set Big Num
  (Variables|Default|SetDistance 1e+04)
  (bind _outactors (Actor|GetAllActorsOfClass "/Game/BluePrints/Zombie/Zombie.Zombie_C"))
  (for _array_element _outactors
    (if (< (Math|Vector|VectorLengthXY (- (Transformation|GetActorLocation _array_element) (Transformation|GetActorLocation))) (Variables|Default|GetDistance))
      (Variables|Default|SetDistance (Math|Vector|VectorLengthXY (- (Transformation|GetActorLocation _array_element) (Transformation|GetActorLocation)))))))