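; LobbyGM is the multiplayer lobby game mode, tracking joined players, their readiness and the selected map until server travel to WaveMap.
; On login it pulls server settings from GameInfoInstance, initializes the LobbyPC menu and possesses a character spawned at a random PlayerStart.
; Joins and logouts rebroadcast player info through each LobbyPC, refresh the host's kick list and recompute CanWeStart.
; It also pushes map changes to all clients and handles kicks.
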(event Custom|RespawnPlayer
  (params (PlayerController :type Player%20Controller%20Object%20Reference))
  (bind _returnvalue (Pawn|GetControlledPawn PlayerController))
  (bind _spawnpoints (Variables|Default|GetSpawnPoints))
  (Utilities|IsValid _returnvalue
    (:Is%20Valid
      (Actor|DestroyActor _returnvalue))
    (:Is%20Not%20Valid
      _))
  (bind _returnvalue_2 (Game|SpawnActorfromClass "/Game/ThirdPerson/Blueprints/BP_ThirdPersonCharacter.BP_ThirdPersonCharacter_C" (Transformation|GetActorTransform (Utilities|Array|Get(acopy) _spawnpoints (Math|Random|RandomIntegerinRange 0 (- (Utilities|Array|Length _spawnpoints) 1)))) "Undefined" "MultiplyWithRoot" 0 0))
  (Pawn|Possess PlayerController _returnvalue_2)
  (CallFunction|EveryoneUpdate))

(event Custom|EveryoneUpdate
  (bind _allplayercontrollers (Variables|Default|GetAllPlayerControllers))
  (bind _output_get (Variables|Default|SetCurrentPlayers (Utilities|Array|Length (Variables|Default|GetAllPlayerControllers))))
  (if (> _output_get 0)
    (Utilities|Array|Clear (Variables|Default|GetConnectedPlayers))
    (for _array_element _allplayercontrollers
      (bind _aslobby_pc (Utilities|Casting|CastToLobbyPC _array_element))
      (Utilities|Array|Add (Variables|Default|GetConnectedPlayers) (Variables|/Game/BluePrints/Basement/LobbyPC.LobbyPC_C|GetPlayerSettings _aslobby_pc))
      (Default|UpdateNumOfPlayers _aslobby_pc (Variables|Default|GetCurrentPlayers) (Variables|Default|GetMaxPlayer)))
    (for _array_element_2 _allplayercontrollers
      (bind _aslobby_pc_2 (Utilities|Casting|CastToLobbyPC _array_element_2))
      (Default|AddPlayerInfo _aslobby_pc_2 (Variables|Default|GetConnectedPlayers))
      (CallFunction|AddtoKickList))
    (bind _array_element_3 (Utilities|Array|ForEachLoopwithBreak (Variables|Default|GetConnectedPlayers))
      (:LoopBody
        (if (Utilities|Enum|Equal(Enum) (.MyPlayerStatus (Utilities|Struct|BreakPlayerInfo _array_element_3)) (Utilities|Text|MakeLiteralText "Not Ready"))
          (Variables|Default|SetCanWeStart? false)
          (CallFunction|CannotStart)
          (else
            (Variables|Default|SetCanWeStart? true)))))))

(event Custom|AddToKickList
  (bind _aslobby_pc (Utilities|Casting|CastToLobbyPC (Game|GetPlayerController 0)))
  (Utilities|IsValid (Variables|/Game/BluePrints/Basement/LobbyPC.LobbyPC_C|GetLobbyMenuWBP _aslobby_pc)
    (:Is%20Valid
      (if (Widget|IsVisible (Variables|/Game/BluePrints/UI/LobbyMenu.LobbyMenu_C|GetGameSettings (Variables|/Game/BluePrints/Basement/LobbyPC.LobbyPC_C|GetLobbyMenuWBP _aslobby_pc)))
        (Default|FillPlayerInfo (Variables|/Game/BluePrints/UI/LobbyMenu.LobbyMenu_C|GetGameSettings (Variables|/Game/BluePrints/Basement/LobbyPC.LobbyPC_C|GetLobbyMenuWBP _aslobby_pc)))))))

(event Custom|CannotStart
  (Utilities|Array|ForEachLoopwithBreak (Variables|Default|GetConnectedPlayers)) ; enters at Break
)

(event Custom|ServerUpdateGameSettings
  (params (MapImage :type Texture%202D%20Object%20Reference) (MapName :type Text) (MapDifficulty :type Text) (MapID :type Integer))
  (Variables|Default|SetGM_MapImage MapImage)
  (Variables|Default|SetGM_MapName MapName)
  (Variables|Default|SetGM_MapDifficulty MapDifficulty)
  (Variables|Default|SetGM_MapID MapID)
  (for _array_element (Variables|Default|GetAllPlayerControllers)
    (bind _aslobby_pc (Utilities|Casting|CastToLobbyPC _array_element))
    (Default|UpdateLobbySettings _aslobby_pc (Variables|Default|GetGM_MapImage) (Variables|Default|GetGM_MapName) (Variables|Default|GetGM_MapDifficulty))))

(event Custom|LaunchTheGame
  ;[1 1 1] If Map added? change to Node switch add too
  (switch int (Variables|Default|GetGM_MapID)
    (:0
      (Development|ExecuteConsoleCommand "servertravel /Game/Maps/WaveMap" (Game|GetPlayerController 0)))))

(event Custom|YouHaveBeenKick
  (params (PlayerID :type Integer))
  (Default|Kicked (.AsLobby%20PC (Utilities|Casting|CastToLobbyPC (Utilities|Array|Get(acopy) (Variables|Default|GetAllPlayerControllers) PlayerID)))))

(event EventPostLogin
  (params (NewPlayer :type Player%20Controller%20Object%20Reference))
  (Networking|SwitchHasAuthority
    (:Authority
      (Utilities|Array|Add (Variables|Default|GetAllPlayerControllers) NewPlayer)
      (bind _outactors (Actor|GetAllActorsOfClass "/Script/Engine.PlayerStart"))
      (Variables|Default|SetSpawnPoints _outactors)
      (bind _asgame_info_instance (Utilities|Casting|CastToGameInfoInstance (Game|GetGameInstance)))
      (Variables|Default|SetServerName (Variables|/Game/BluePrints/Basement/GameInfoInstance.GameInfoInstance_C|GetServerName _asgame_info_instance))
      (Variables|Default|SetMaxPlayer (Variables|/Game/BluePrints/Basement/GameInfoInstance.GameInfoInstance_C|GetMaxPlayers _asgame_info_instance))
      (bind _aslobby_pc (Utilities|Casting|CastToLobbyPC NewPlayer))
      (Default|InitialSetup _aslobby_pc)
      (Default|SetupLobbyMenu _aslobby_pc (Variables|Default|GetServerName))
      (Default|UpdateLobbySettings _aslobby_pc (Variables|Default|GetGM_MapImage) (Variables|Default|GetGM_MapName) (Variables|Default|GetGM_MapDifficulty))
      (CallFunction|RespawnPlayer NewPlayer))))

(event EventOnLogout
  (params (ExitingController :type Controller%20Object%20Reference))
  (bind (_array_element _array_index) (Utilities|Array|ForEachLoopwithBreak (Variables|Default|GetAllPlayerControllers) :!label _label)
    (:LoopBody
      (if (== _array_element ExitingController)
        (goto _label Break)))
    (:Completed
      (Utilities|Array|RemoveIndex (Variables|Default|GetAllPlayerControllers) _array_index)
      (Utilities|Array|RemoveIndex (Variables|Default|GetConnectedPlayers) _array_index)
      (CallFunction|EveryoneUpdate))))

(fn ConstructionScript)