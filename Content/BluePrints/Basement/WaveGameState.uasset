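; WaveGameState is a Game State that tracks wave number, wave state, preparation countdown, and monster and boss counts for a wave-based mode.
; SetWaveState passes the state through a companion SC event, then broadcasts the change after a short delay, while Tick runs the countdown.
; Decrement functions notify TestGameMode and fire kill events when a current count is zero in a specific state.
; The boss decrement lowers the total but tests the current count.
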(event Custom|OnWaveChange_Event)

(event Custom|SetWaveState
  (params (NewState :type WaveState%20Enum :default "NewEnumerator0"))
  (bind _output_get (Variables|Default|SetWaveState NewState))
  (CallFunction|SCSetWaveState _output_get)
  (Utilities|FlowControl|Delay 0.5)
  (Default|CallOnWaveChange))

(event Custom|SC_SetWaveState
  (params (NewState :type WaveState%20Enum :default "NewEnumerator0"))
  (Variables|Default|SetWaveState NewState))

(event EventBeginPlay)

(event EventTick
  (params (DeltaSeconds :type Float%20%28single-precision%29))
  (if (Utilities|Enum|Equal(Enum) (Variables|Default|GetWaveState) "NewEnumerator0")
    (Variables|Default|SetPrepareTime (- (Variables|Default|GetPrepareTime) DeltaSeconds))))

(fn ConstructionScript)

(fn IncrementWave
  (Math|Integer|IncrementInt (Variables|Default|GetCurrentWave)
    (:%20%20
      (Default|CallOnWaveStart))))

(fn IncrementMonsterCount
  (Math|Integer|IncrementInt (Variables|Default|GetCurrentMonsterInWave)))

(fn DecrementMonsterCount
  (Math|Integer|DecrementInt (Variables|Default|GetCurrentMonsterInWave)
    (:%20%20
      (if (and (== (Variables|Default|GetCurrentMonsterInWave) 0) (Utilities|Enum|Equal(Enum) (Variables|Default|GetWaveState) "NewEnumerator2"))
        (bind _astest_game_mode (Utilities|Casting|CastToTestGameMode (Game|GetGameMode)))
        (Default|AllEnemyDead _astest_game_mode)
        (Default|CallAllEnemyKilled)))))

(fn SetTotalMonster
  (params (TotalMonsterNumber :type Integer))
  (Variables|Default|SetTotalMonsterInWave TotalMonsterNumber))

(fn SetTotalWave
  (params (TotalWave :type Integer))
  (Variables|Default|SetTotalWave TotalWave))

(fn SetPrepareTime
  (params (InputTime :type Float%20%28double-precision%29))
  (Variables|Default|SetPrepareTime InputTime))

(fn OnRepWaveState)

(fn SetTotalBoss
  (params (TotalBossNum :type Integer))
  (Variables|Default|SetTotalBossMonsterInWave TotalBossNum))

(fn IncrementBossMonsterCount
  (Math|Integer|IncrementInt (Variables|Default|GetCurrentBossMonsterInWave)))

(fn DecrementBossMonsterCount
  (Math|Integer|DecrementInt (Variables|Default|GetTotalBossMonsterInWave)
    (:%20%20
      (if (and (== (Variables|Default|GetCurrentBossMonsterInWave) 0) (Utilities|Enum|Equal(Enum) (Variables|Default|GetWaveState) "NewEnumerator2"))
        (bind _astest_game_mode (Utilities|Casting|CastToTestGameMode (Game|GetGameMode)))
        (Default|BossKilled _astest_game_mode)
        (Default|CallBossKilled)))))