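; Game mode for a multiplayer zombie wave game that manages connected players, respawning and the wave cycle.
; Joins, controller swaps and logouts rebuild a player-settings list that is pushed to every ZombieController.
; Respawns claim the first untagged PlayerStart, marking it used, then spawn and possess a new Zombie pawn.
; WaveGameState holds wave progress; timed prepare phases lead into monster spawning, restarting when all enemies die until the final wave.
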(event Custom|RespawnPlayer
  (params (PlayerController :type Player%20Controller%20Object%20Reference))
  (bind _returnvalue (Pawn|GetControlledPawn PlayerController))
  (bind _array_element (Utilities|Array|ForEachLoopwithBreak (Variables|GameInfo|GetSpawnPoints) :!label _label)
    (:LoopBody
      (if (== (Variables|/Script/Engine.PlayerStart|GetPlayerStartTag _array_element) "")
        (Variables|/Script/Engine.PlayerStart|SetPlayerStartTag _array_element "Been")
        (goto _label Break)))
    (:Completed
      (Utilities|IsValid _returnvalue
        (:Is%20Valid
          (Actor|DestroyActor _returnvalue))
        (:Is%20Not%20Valid
          _))
      (bind _returnvalue_2 (Game|SpawnActorfromClass "/Game/BluePrints/Zombie/Zombie.Zombie_C" (Transformation|GetActorTransform _array_element) "Undefined" "MultiplyWithRoot" 0 0))
      (Pawn|Possess PlayerController _returnvalue_2))))

(event Custom|AllEnemyDead
  (bind _preparetime (Variables|Default|GetPrepareTime))
  (Default|SetWaveState (Variables|Default|GetWaveGameState) "NewEnumerator0")
  (Utilities|Time|SetTimerbyFunctionName 0 "StartNextWave" _preparetime)
  (Default|SetPrepareTime (Variables|Default|GetWaveGameState) _preparetime))

(event Custom|UpdatePlayers
  (bind _allplayercontroller (Variables|GameInfo|GetAllPlayerController))
  (if (> (Utilities|Array|Length (Variables|GameInfo|GetAllPlayerController)) 0)
    (Utilities|Array|Clear (Variables|Default|GetConnectedPlayers))
    (for _array_element _allplayercontroller
      (bind _aszombie_controller (Utilities|Casting|CastToZombieController _array_element))
      (Utilities|Array|Add (Variables|Default|GetConnectedPlayers) (Variables|/Game/BluePrints/Basement/ZombieController.ZombieController_C|GetPlayerSettings _aszombie_controller)))
    (for _array_element_2 _allplayercontroller
      (bind _aszombie_controller_2 (Utilities|Casting|CastToZombieController _array_element_2))
      (Default|UpdatePlayerInfo _aszombie_controller_2 (Variables|Default|GetConnectedPlayers)))))

(event EventBeginPlay
  (bind _initialtime (Variables|Default|GetInitialTime))
  (bind _aswave_game_state (Utilities|Casting|CastToWaveGameState (Game|GetGameState)))
  (Variables|Default|SetWaveGameState _aswave_game_state)
  (bind _outactors (Actor|GetAllActorsOfClass "/Script/Engine.PlayerStart"))
  (Variables|GameInfo|SetSpawnPoints _outactors)
  (bind _aszombie_controller (Utilities|Casting|CastToZombieController (Game|GetPlayerController 0)))
  (Default|SetupWidgets _aszombie_controller)
  (Default|SetTotalWave (Variables|Default|GetWaveGameState) 3)
  (Default|SetWaveState (Variables|Default|GetWaveGameState) "NewEnumerator0")
  (Utilities|Time|SetTimerbyFunctionName 0 "StartNextWave" _initialtime)
  (Default|SetPrepareTime (Variables|Default|GetWaveGameState) _initialtime))

(event EventPostLogin
  (params (NewPlayer :type Player%20Controller%20Object%20Reference))
  (Utilities|Array|Add (Variables|GameInfo|GetAllPlayerController) NewPlayer)
  (CallFunction|UpdatePlayers))

(event EventOnSwapPlayerControllers
  (params (OldPC :type Player%20Controller%20Object%20Reference) (NewPC :type Player%20Controller%20Object%20Reference))
  (Utilities|Array|Add (Variables|GameInfo|GetAllPlayerController) NewPC)
  (CallFunction|UpdatePlayers))

(event EventOnLogout
  (params (ExitingController :type Controller%20Object%20Reference))
  (bind (_array_element _array_index) (Utilities|Array|ForEachLoopwithBreak (Variables|GameInfo|GetAllPlayerController) :!label _label)
    (:LoopBody
      (if (== _array_element ExitingController)
        (goto _label Break)))
    (:Completed
      (Utilities|Array|RemoveIndex (Variables|GameInfo|GetAllPlayerController) _array_index)
      (CallFunction|UpdatePlayers))))

(fn ConstructionScript)

(fn StartNextWave
  (bind _wavegamestate (Variables|Default|GetWaveGameState))
  (bind _wavegamestate_2 (Variables|Default|GetWaveGameState))
  (if (< (Variables|/Game/BluePrints/Basement/WaveGameState.WaveGameState_C|GetCurrentWave _wavegamestate_2) (Variables|/Game/BluePrints/Basement/WaveGameState.WaveGameState_C|GetTotalWave _wavegamestate_2))
    (Default|IncrementWave _wavegamestate)
    (Default|SetWaveState _wavegamestate "NewEnumerator1")
    (Default|SetTotalMonster _wavegamestate (Utilities|Array|Get(acopy) (Variables|Default|GetWaveMonsterNumber) (Variables|/Game/BluePrints/Basement/WaveGameState.WaveGameState_C|GetCurrentWave (Variables|Default|GetWaveGameState))))
    (Default|CallCallSpawnMonsters)))