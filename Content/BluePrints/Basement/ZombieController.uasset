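; Player controller for the Zombie pawn in a multiplayer wave game, handling movement, look, HUD widgets and text chat.
; On local BeginPlay it loads saved player settings, passes them on for a GameMode respawn and binds GameState wave events that toggle the wave UI.
; It creates menu, health, chat, scoreboard and wave widgets, with keys toggling them.
; Chat relays through the GameMode's controller list, and EndPlay destroys the session.
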(event Custom|GetChatMessage
  (params (TextToSend :type Text))
  (Variables|Chatting|SetSenderText TextToSend)
  (Variables|Chatting|SetSenderName (.MyPlayerName (Utilities|Struct|BreakPlayerInfo (Variables|Default|GetPlayerSettings))))
  (bind _astest_game_mode (Utilities|Casting|CastToTestGameMode (Game|GetGameMode)))
  (for _array_element (Variables|/Game/BluePrints/Basement/TestGameMode.TestGameMode_C|GetAllPlayerController _astest_game_mode)
    (bind _aszombie_controller (Utilities|Casting|CastToZombieController _array_element))
    (CallFunction|UpdateChat _aszombie_controller (Variables|Chatting|GetSenderName) (Variables|Chatting|GetSenderText))))

(event Custom|UpdateChat
  (params (SenderName :type Text) (SenderText :type Text))
  (Default|UpdateChatWindow (Variables|/Game/BluePrints/UI/InGameChat.InGameChat_C|GetGamePlayChat (Variables|Widget|GetChatWBP)) SenderName SenderText))

(event Custom|PassCharacterInfoToServer
  (params (PlayerSettingInfo :type Player%20Info%20Structure))
  (Variables|Default|SetPlayerSettings PlayerSettingInfo)
  (bind _astest_game_mode (Utilities|Casting|CastToTestGameMode (Game|GetGameMode)))
  (Default|RespawnPlayer _astest_game_mode self)
  (CallFunction|SetupWidgets))

(event Custom|SetupWidgets
  (CallFunction|SetupinGameMenu)
  (CallFunction|SetupHealthUI)
  (CallFunction|SetupChattingUI)
  (CallFunction|SetupScoreboardUI)
  (CallFunction|SetupWaveUI))

(event Custom|StartWave
  (bind _wavewbp (Variables|Widget|GetWaveWBP))
  (Utilities|IsValid _wavewbp
    (:Is%20Valid
      (Widget|SetVisibility _wavewbp "Hidden"))))

(event Custom|WaveStateChanged
  (bind _wavewbp (Variables|Widget|GetWaveWBP))
  (if (Utilities|Enum|Equal(Enum) (Variables|/Game/BluePrints/Basement/WaveGameState.WaveGameState_C|GetWaveState (Variables|Default|GetGameState)) "NewEnumerator0")
    (Utilities|IsValid _wavewbp
      (:Is%20Valid
        (Widget|SetVisibility _wavewbp "Visible")))))

(event Custom|UpdatePlayerInfo
  (params (GameModePlayerInfo :type Array%20of%20Player%20Info%20Structures))
  (bind _scoreboardwbp (Variables|Widget|GetScoreboardWBP))
  (Variables|Default|SetAllConnectedPlayers GameModePlayerInfo)
  (Utilities|IsValid _scoreboardwbp
    (:Is%20Valid
      (Default|UpdatePlayerInfo _scoreboardwbp (Variables|Default|GetAllConnectedPlayers)))))

(event Input|EnhancedActionEvents|EnhancedInputActionIA_Rotate
  (params (ActionValue :type Vector%202D%20Structure) (ElapsedSeconds :type Float%20%28double-precision%29) (TriggeredSeconds :type Float%20%28double-precision%29) (InputAction :type Input%20Action%20Object%20Reference :default "/Game/BluePrints/InputAction/IA_Rotate.IA_Rotate"))
  (Class|PlayerController|AddYawInput (.x ActionValue))
  (Class|PlayerController|AddPitchInput (.y ActionValue)))

(event Input|EnhancedActionEvents|EnhancedInputActionIA_Move
  (params (ActionValue :type Vector%202D%20Structure) (ElapsedSeconds :type Float%20%28double-precision%29) (TriggeredSeconds :type Float%20%28double-precision%29) (InputAction :type Input%20Action%20Object%20Reference :default "/Game/BluePrints/InputAction/IA_Move.IA_Move"))
  (bind _returnvalue (Pawn|GetControlRotation :!class /Script/Engine.Controller))
  (bind _returnvalue_2 (Pawn|GetControlledPawn))
  (bind _returnvalue_3 (Math|Rotator|MakeRotator 0.0 0.0 (.yaw _returnvalue)))
  (Pawn|Input|AddMovementInput _returnvalue_2 (Math|Vector|GetForwardVector _returnvalue_3) (.x ActionValue) false)
  (Pawn|Input|AddMovementInput _returnvalue_2 (Math|Vector|GetRightVector _returnvalue_3) (.y ActionValue) false))

(event EventEndPlay
  (params (EndPlayReason :type EEndPlayReason%20Enum :default "Destroyed"))
  (|DestroySession self))

(event EventBeginPlay
  (if (Pawn|IsLocalController)
    (Viewport|RemoveAllWidgets)
    (Input|SetInputModeGameOnly self false)
    (CallFunction|LoadGame)
    (Input|AddMappingContext (PlayerController|LocalPlayerSubsystems|GetEnhancedInputLocalPlayerSubsystem) "/Game/BluePrints/InputAction/IMC.IMC" 0 "(bIgnoreAllPressedKeysUntilRelease=True,bForceImmediately=False,bNotifyUserSettings=False)")
    (CallFunction|PassCharacterInfotoServer (Variables|Default|GetPlayerSettings))
    (bind _aswave_game_state (Utilities|Casting|CastToWaveGameState (Game|GetGameState)))
    (Variables|Default|SetGameState _aswave_game_state)
    (EventDispatchers|BindEventtoOnWaveStart (Variables|Default|GetGameState) (delegate Custom|StartWave))
    (EventDispatchers|BindEventtoOnWaveChange (Variables|Default|GetGameState) (delegate Custom|WaveStateChanged))))

(event Input|KeyboardEvents|M
  (params (Key :type Key%20Structure :default "None"))
  (:Pressed
    (Default|PressedPause (Variables|Widget|GetInGameMenu))))

(event Input|KeyboardEvents|T
  (params (Key :type Key%20Structure :default "None"))
  (bind _chatwbp (Variables|Widget|GetChatWBP))
  (:Pressed
    (Utilities|FlowControl|FlipFlop
      (:A
        (Widget|SetVisibility _chatwbp "Visible")
        (Variables|Default|SetbShowMouseCursor true)
        (Input|SetInputModeGameandUI self _chatwbp "DoNotLock" true false))
      (:B
        (Widget|SetVisibility (Variables|Widget|GetChatWBP) "Hidden")
        (Variables|Default|SetbShowMouseCursor false)
        (Input|SetInputModeGameOnly self false)))))

(event Input|KeyboardEvents|Escape
  (params (Key :type Key%20Structure :default "None"))
  (:Pressed
    (Default|PressedPause (Variables|Widget|GetInGameMenu))))

(event Input|KeyboardEvents|Tab
  (params (Key :type Key%20Structure :default "None"))
  (bind _scoreboardwbp (Variables|Widget|GetScoreboardWBP))
  (bind _scoreboardwbp_2 (Variables|Widget|GetScoreboardWBP))
  (:Pressed
    (Utilities|IsValid _scoreboardwbp_2
      (:Is%20Valid
        (Widget|SetVisibility _scoreboardwbp_2 "Visible"))))
  (:Released
    (Utilities|IsValid _scoreboardwbp
      (:Is%20Valid
        (Widget|SetVisibility _scoreboardwbp "Hidden")))))

(fn ConstructionScript)

(fn SetupChattingUI
  (Utilities|IsValid (Variables|Widget|GetChatWBP)
    (:Is%20Valid
      _)
    (:Is%20Not%20Valid
      (bind _returnvalue (UserInterface|CreateWidget "/Game/BluePrints/UI/InGameChat.InGameChat_C" self))
      (bind _output_get (Variables|Widget|SetChatWBP _returnvalue))))
  (UserInterface|Viewport|AddtoViewport _output_get 0)
  (Widget|SetVisibility _output_get "Hidden"))

(fn LoadGame
  (bind _returnvalue (SaveGame|LoadGamefromSlot (Variables|SaveLoad|GetPlayerSettingsSave)))
  (bind _asplayer_save_game (Utilities|Casting|CastToPlayerSaveGame _returnvalue))
  (Variables|Default|SetPlayerSettings (Variables|/Game/BluePrints/Basement/PlayerSaveGame.PlayerSaveGame_C|GetS_PlayerInfo _asplayer_save_game)))

(fn SetupinGameMenu
  (bind _self self)
  (Utilities|IsValid (Variables|Widget|GetInGameMenu)
    (:Is%20Valid
      _)
    (:Is%20Not%20Valid
      (bind _returnvalue (UserInterface|CreateWidget "/Game/BluePrints/UI/InGameMenu.InGameMenu_C" _self _self))
      (bind _output_get (Variables|Widget|SetInGameMenu _returnvalue))))
  (UserInterface|Viewport|AddtoViewport _output_get 0)
  (Widget|SetVisibility _output_get "Hidden"))

(fn SetupHealthUI
  (Utilities|IsValid (Variables|Widget|GetPlayerUI)
    (:Is%20Valid
      _)
    (:Is%20Not%20Valid
      (bind _aszombie (Utilities|Casting|CastToZombie (Pawn|GetControlledPawn)))
      (bind _returnvalue (UserInterface|CreateWidget "/Game/BluePrints/UI/Zombie_UI.Zombie_UI_C" self _aszombie))
      (bind _output_get (Variables|Widget|SetPlayerUI _returnvalue))))
  (UserInterface|Viewport|AddtoViewport _output_get 0))

(fn SetupScoreboardUI
  (Utilities|IsValid (Variables|Widget|GetScoreboardWBP)
    (:Is%20Valid
      _)
    (:Is%20Not%20Valid
      (bind _returnvalue (UserInterface|CreateWidget "/Game/BluePrints/UI/Scoreboard.Scoreboard_C" self))
      (bind _output_get (Variables|Widget|SetScoreboardWBP _returnvalue))))
  (UserInterface|Viewport|AddtoViewport _output_get 0)
  (Widget|SetVisibility _output_get "Hidden"))

(fn SetupWaveUI
  (Utilities|IsValid (Variables|Widget|GetWaveWBP)
    (:Is%20Valid
      _)
    (:Is%20Not%20Valid
      (bind _returnvalue (UserInterface|CreateWidget "/Game/BluePrints/UI/Clear_UI.Clear_UI_C" self))
      (bind _output_get (Variables|Widget|SetWaveWBP _returnvalue))))
  (UserInterface|Viewport|AddtoViewport _output_get 0)
  (Widget|SetVisibility _output_get "Hidden"))