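; Player controller for the multiplayer lobby that drives the lobby menu, chat and player list.
; It passes player settings to LobbyGM for an update to everyone and relays chat through LobbyGM's controller list.
; Events fill the menu with players, map info and player count, or swap it for a loading screen.
; T toggles menu visibility; being kicked opens the title level, and both kick and EndPlay destroy the session.
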(event Custom|InitialSetup
  (CallFunction|SaveGameCheck)
  (CallFunction|CallUpdate (Variables|Default|GetPlayerSettings) false))

(event Custom|CallUpdate
  (params (PlayerInfo :type Player%20Info%20Structure) (ChangeStatus? :type Boolean))
  (Variables|Default|SetPlayerSettings PlayerInfo)
  (Default|EveryoneUpdate (.AsLobby%20GM (Utilities|Casting|CastToLobbyGM (Game|GetGameMode)))))

(event Custom|SetupLobbyMenu
  (params (ServerName :type Text))
  (Variables|Default|SetbShowMouseCursor true)
  (bind _returnvalue (UserInterface|CreateWidget "/Game/BluePrints/UI/LobbyMenu.LobbyMenu_C" 0 ServerName))
  (bind _output_get (Variables|Default|SetLobbyMenuWBP _returnvalue))
  (UserInterface|Viewport|AddtoViewport _output_get 0)
  (Input|SetInputModeGameandUI self _output_get "DoNotLock" true false))

(event Custom|AddPlayerInfo
  (params (ConnectedPlayerInfo :type Array%20of%20Player%20Info%20Structures))
  (bind _lobbymenuwbp (Variables|Default|GetLobbyMenuWBP))
  (Variables|Default|SetAllConnectedPlayers ConnectedPlayerInfo)
  (Utilities|IsValid _lobbymenuwbp
    (:Is%20Valid
      (Default|ClearPlayerList _lobbymenuwbp)
      (for _array_element (Variables|Default|GetAllConnectedPlayers)
        (Default|UpdatePlayerWindow (Variables|Default|GetLobbyMenuWBP) _array_element)))))

(event Custom|UpdateLobbySettings
  (params (MapImage :type Texture%202D%20Object%20Reference) (MapName :type Text) (MapTime :type Text))
  (bind _lobbymenuwbp (Variables|Default|GetLobbyMenuWBP))
  (Variables|/Game/BluePrints/UI/LobbyMenu.LobbyMenu_C|SetMapImage _lobbymenuwbp MapImage)
  (Variables|/Game/BluePrints/UI/LobbyMenu.LobbyMenu_C|SetMapName _lobbymenuwbp MapName)
  (Variables|/Game/BluePrints/UI/LobbyMenu.LobbyMenu_C|SetMapTime _lobbymenuwbp MapTime))

(event Custom|ShowLoadingScreen
  (Widget|RemovefromParent (Variables|Default|GetLobbyMenuWBP))
  (bind _returnvalue (UserInterface|CreateWidget "/Game/BluePrints/UI/LoadingScreen.LoadingScreen_C" self))
  (UserInterface|Viewport|AddtoViewport _returnvalue 0))

(event Custom|UpdateNumOfPlayers
  (params (CurrentPlayers :type Integer) (MaxPlayers :type Integer))
  (bind _lobbymenuwbp (Variables|Default|GetLobbyMenuWBP))
  (Utilities|IsValid _lobbymenuwbp
    (:Is%20Valid
      (Variables|/Game/BluePrints/UI/LobbyMenu.LobbyMenu_C|SetPlayersDisplay _lobbymenuwbp (Utilities|Text|FormatText "{CurrentPlayers} / {MaxPlayers}" (Utilities|Text|ToText(Integer) CurrentPlayers) (Utilities|Text|ToText(Integer) MaxPlayers))))))

(event Custom|Kicked
  (Game|OpenLevel(byName) "TitleLevel")
  (|DestroySession self))

(event Custom|GetChatMessage
  (params (TextToSend :type Text))
  (Variables|Default|SetSenderText TextToSend)
  (Variables|Default|SetSenderName (.MyPlayerName (Utilities|Struct|BreakPlayerInfo (Variables|Default|GetPlayerSettings))))
  (bind _aslobby_gm (Utilities|Casting|CastToLobbyGM (Game|GetGameMode)))
  (for _array_element (Variables|/Game/BluePrints/Basement/LobbyGM.LobbyGM_C|GetAllPlayerControllers _aslobby_gm)
    (bind _aslobby_pc (Utilities|Casting|CastToLobbyPC _array_element))
    (CallFunction|ChatUpdate _aslobby_pc (Variables|Default|GetSenderName) (Variables|Default|GetSenderText))))

(event Custom|ChatUpdate
  (params (Sender :type Text) (Text :type Text))
  (Default|UpdateChatWindow (Variables|/Game/BluePrints/UI/LobbyMenu.LobbyMenu_C|GetChatWindow (Variables|Default|GetLobbyMenuWBP)) Sender Text))

(event EventEndPlay
  (params (EndPlayReason :type EEndPlayReason%20Enum :default "Destroyed"))
  (|DestroySession self))

(event Input|KeyboardEvents|T
  (params (Key :type Key%20Structure :default "None"))
  (bind _lobbymenuwbp (Variables|Default|GetLobbyMenuWBP))
  (:Pressed
    (Utilities|FlowControl|FlipFlop
      (:A
        (Widget|SetVisibility _lobbymenuwbp "Hidden"))
      (:B
        (Widget|SetVisibility _lobbymenuwbp "Visible")))))

(fn ConstructionScript)

(fn SaveGameCheck)