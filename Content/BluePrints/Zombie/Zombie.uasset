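; Player-controlled character in the Zombie folder that picks up, holsters and fires up to two rifles, with sprint, reload and death.
; Input and Tick route through paired CS_/SC_ events, apparently server and multicast RPCs.
; A HandArm state selects the active RifleSlot and its socket attachment, while an RPM-based timer repeats camera line-trace shots that apply damage and spawn explosion effects.
; Damage is handled on the server, triggering death animation and UI.
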(event OnComponentBeginOverlap(CapsuleComponent)
  (params (OverlappedComponent :type Primitive%20Component%20Object%20Reference) (OtherActor :type Actor%20Object%20Reference) (OtherComp :type Primitive%20Component%20Object%20Reference) (OtherBodyIndex :type Integer) (bFromSweep :type Boolean) (SweepResult :type Hit%20Result%20Structure%20%28by%20ref%29))
  (bind _can_ (Class|Handle|CanPick(Message) OtherActor))
  (if _can_
    (Variables|Default|SetCan%20Pick? _can_)
    (Variables|Default|SetPickable%20Actor OtherActor)
    (Rendering|SetVisibility (Variables|Default|GetTextRender) true false)))

(event OnComponentEndOverlap(CapsuleComponent)
  (params (OverlappedComponent :type Primitive%20Component%20Object%20Reference) (OtherActor :type Actor%20Object%20Reference) (OtherComp :type Primitive%20Component%20Object%20Reference) (OtherBodyIndex :type Integer))
  (bind _can_ (Class|Handle|CanPick(Message) OtherActor))
  (if _can_
    (Variables|Default|SetCan%20Pick? false)
    (Variables|Default|SetPickable%20Actor 0)
    (Rendering|SetVisibility (Variables|Default|GetTextRender) false false)))

(event Custom|CS_Fire
  (CallFunction|Fire)
  (CallFunction|SCFire))

(event Custom|SC_Fire)

(event Custom|CS_Rifle1
  (CallFunction|SCRifle1))

(event Custom|SC_Rifle1
  (CallFunction|Pressed1))

(event Custom|CS_Rifle2
  (CallFunction|SCRifle2))

(event Custom|SC_Rifle2
  (CallFunction|Pressed2))

(event Custom|SC_InitialSetting
  (CallFunction|InitialSetting))

(event Custom|CS_InitialSetting
  (CallFunction|InitialSetting)
  (CallFunction|SCInitialSetting))

(event Custom|SC_FireAnim
  (Animation|PlayAnimMontage "/Game/BluePrints/Zombie/RifleMontage.RifleMontage" 1.0 "Fire"))

(event Custom|SC_SpawnExplosion
  (params (Location :type Vector))
  (Effects|SpawnEmitteratLocation "/Game/StarterContent/Particles/P_Explosion.P_Explosion" Location "0, 0, 0" "0.300000,0.300000,0.300000"))

(event Custom|SC_PlayDeadAnim
  (Components|Animation|PlayAnimation (Variables|Character|GetMesh) "/Game/ZombieAsset/ZombieAnimation/Death.Death" false)
  (Collision|SetCollisionEnabled (Variables|Collision|GetCapsuleComponent) "NoCollision")
  (Pawn|Components|CharacterMovement|SetMovementMode (Variables|Character|GetCharacterMovement) "MOVE_None" 0))

(event Custom|PopUpDeadUI
  (Input|DisableInput (Game|Player|GetPlayerPawn 0) 0)
  (bind _returnvalue (UserInterface|CreateWidget "/Game/BluePrints/UI/Die_UI.Die_UI_C"))
  (UserInterface|Viewport|AddtoViewport _returnvalue 0))

(event Custom|CS_PickUp
  (bind _index (CallFunction|PickUpWeapon))
  (CallFunction|SCPickUp _index))

(event Custom|SetHealth
  (params (NewHP :type Float%20%28double-precision%29))
  (Variables|Default|SetHealth NewHP))

(event Custom|CS_PressDash
  (CallFunction|SCPressDash))

(event Custom|CS_ReleaseDash
  (CallFunction|SCReleaseDash))

(event Custom|SC_PressDash
  (Variables|/Script/Engine.CharacterMovementComponent|SetMaxWalkSpeed (Variables|Character|GetCharacterMovement) 9e+02))

(event Custom|SC_ReleaseDash
  (Variables|/Script/Engine.CharacterMovementComponent|SetMaxWalkSpeed (Variables|Character|GetCharacterMovement) 6e+02))

(event Custom|SC_PickUp
  (params (Index :type Integer))
  (if (>= Index 0)
    (CallFunction|StoreRifle (Variables|Default|GetHand%20Arm))
    (if (== Index 0)
      (CallFunction|UseRifle "NewEnumerator1")
      (elif (== Index 1)
        (CallFunction|UseRifle "NewEnumerator2")))
    (Variables|Default|SetHolding%20Gun? true)
    (Variables|Default|SetPickable%20Actor 0)
    (Variables|Default|SetCan%20Pick? false)
    (Rendering|SetVisibility (Variables|Default|GetTextRender) false false)
    (Animation|PlayAnimMontage "/Game/BluePrints/Zombie/RifleMontage.RifleMontage" 1.0 "Aim")
    (CallFunction|UpdateUsingRifle)))

(event Custom|CS_Reload
  (CallFunction|SCReload))

(event Custom|SC_Reload
  (Utilities|ReloadMotion))

(event Custom|SC_WaistAnim)

(event Custom|CS_WaistAnim
  (Variables|Default|SetY%20%28Pitch%29 (.Pitch (Math|Rotator|BreakRotator (Pawn|GetControlRotation :!class /Script/Engine.Pawn))))
  (CallFunction|SCWaistAnim))

(event Custom|CS_UpdateTick
  (CallFunction|UpdateinTick)
  (CallFunction|SCUpdateTick))

(event Custom|SC_UpdateTick)

(event Input|EnhancedActionEvents|EnhancedInputActionIA_Jump
  (params (ActionValue :type Boolean) (ElapsedSeconds :type Float%20%28double-precision%29) (TriggeredSeconds :type Float%20%28double-precision%29) (InputAction :type Input%20Action%20Object%20Reference :default "/Game/BluePrints/InputAction/IA_Jump.IA_Jump"))
  (:Started
    (Character|Jump)))

(event EventBeginPlay
  (Rendering|SetVisibility (Variables|Default|GetTextRender) false false)
  (bind _aszombie_controller (Utilities|Casting|CastToZombieController (Game|GetPlayerController 0)))
  (Default|SetupWidgets _aszombie_controller)
  (CallFunction|CSInitialSetting))

(event Game|Damage|EventAnyDamage
  (params (Damage :type Float%20%28single-precision%29) (DamageType :type Damage%20Type%20Object%20Reference) (InstigatedBy :type Controller%20Object%20Reference) (DamageCauser :type Actor%20Object%20Reference))
  (bind _health (Variables|Default|GetHealth))
  (if (Networking|IsServer)
    (CallFunction|SetHealth (- _health Damage))
    (if (<= _health 0.0)
      (CallFunction|SCPlayDeadAnim)
      (CallFunction|PopUpDeadUI)
      (Variables|Default|SetDeath true))))

(event EventTick
  (params (DeltaSeconds :type Float%20%28single-precision%29))
  (CallFunction|CSUpdateTick)
  (CallFunction|CSWaistAnim))

(event Input|MouseEvents|LeftMouseButton
  (params (Key :type Key%20Structure :default "None"))
  (:Pressed
    (if (Variables|Default|GetHolding%20Gun?)
      (if (not (Variables|Default|GetReloading))
        (Variables|Default|SetShooting? true)
        (CallFunction|UpdateUsingRifle)
        (CallFunction|CSFire)
        (bind _returnvalue (Utilities|Time|SetTimerbyFunctionName 0 "CS_Fire" (/ 6e+01 (Variables|/Game/BluePrints/Rifle/BP_RifleBase.BP_RifleBase_C|GetRPM (Variables|Default|GetUsingRifle))) true))
        (Variables|Default|SetTimerHandle _returnvalue))))
  (:Released
    (Variables|Default|SetShooting? false)
    (Utilities|Time|ClearandInvalidateTimerbyHandle (Variables|Default|GetTimerHandle))))

(event Input|MouseEvents|LeftMouseButton
  (params (Key :type Key%20Structure :default "None"))
  ;[1 1 1] Regacy
)

(event Input|KeyboardEvents|R
  (params (Key :type Key%20Structure :default "None"))
  (:Pressed
    (CallFunction|CSReload)))

(event Input|KeyboardEvents|2
  (params (Key :type Key%20Structure :default "None"))
  (:Pressed
    (CallFunction|CSRifle2)))

(event Input|KeyboardEvents|F
  (params (Key :type Key%20Structure :default "None"))
  (:Pressed
    (if (Variables|Default|GetCan%20Pick?)
      (CallFunction|CSPickUp))))

(event Input|KeyboardEvents|LeftShift
  (params (Key :type Key%20Structure :default "None"))
  (:Pressed
    (CallFunction|CSPressDash))
  (:Released
    (CallFunction|CSReleaseDash)))

(event Input|KeyboardEvents|1
  (params (Key :type Key%20Structure :default "None"))
  (:Pressed
    (CallFunction|CSRifle1)))

(event Input|KeyboardEvents|G
  (params (Key :type Key%20Structure :default "None"))
  ;[1 1 1] 버리는거 이게 아닌가
)

(fn ConstructionScript)

(fn Fire
  (bind _camera (Variables|Default|GetCamera))
  (bind _returnvalue (Transformation|GetWorldLocation _camera))
  (CallFunction|UpdateUsingRifle)
  (if (> (Variables|/Game/BluePrints/Rifle/BP_RifleBase.BP_RifleBase_C|GetCurrMag (Variables|Default|GetUsingRifle)) 0)
    (Math|Integer|DecrementInt (Variables|/Game/BluePrints/Rifle/BP_RifleBase.BP_RifleBase_C|GetCurrMag (Variables|Default|GetUsingRifle))
      (:%20%20
        (CallFunction|SCFireAnim)
        (bind (_outhit _returnvalue_2) (Collision|LineTraceByChannel _returnvalue (+ _returnvalue (* (Math|Vector|GetForwardVector (Pawn|GetControlRotation :!class /Script/Engine.Pawn)) 1e+04)) "TraceTypeQuery1" false 0 "None"))
        (if _returnvalue_2
          (CallFunction|SCSpawnExplosion (.Location (Collision|BreakHitResult _outhit)))
          (Game|Damage|ApplyDamage (.HitActor (Collision|BreakHitResult _outhit)) (Variables|/Game/BluePrints/Rifle/BP_RifleBase.BP_RifleBase_C|GetDamage (Variables|Default|GetUsingRifle)) 0 0))))))

(fn PickUpWeapon
  (bind _emptyslotindex (CallFunction|FindEmptyWeaponSlot))
  (if (>= _emptyslotindex 0)
    (bind _asbp_rifle_base (Utilities|Casting|CastToBP_RifleBase (Variables|Default|GetPickable%20Actor)))
    (bind _ok (Default|Grab _asbp_rifle_base))
    (if _ok
      (Utilities|Array|SetArrayElem (Variables|Default|GetRifleSlot) _emptyslotindex _asbp_rifle_base)
      (Variables|Default|SetHolding%20Gun? true)
      (Variables|Default|SetPickable%20Actor 0)
      (Variables|Default|SetCan%20Pick? false)
      (Rendering|SetVisibility (Variables|Default|GetTextRender) false false)
      (CallFunction|StoreRifle (Variables|Default|GetHand%20Arm))
      (if (== _emptyslotindex 0)
        (CallFunction|UseRifle "NewEnumerator1")
        (Animation|PlayAnimMontage "/Game/BluePrints/Zombie/RifleMontage.RifleMontage" 1.0 "Aim" :!label _label)
        (CallFunction|UpdateUsingRifle)
        (elif (== _emptyslotindex 1)
          (CallFunction|UseRifle "NewEnumerator2")
          (goto _label)
          (else
            _)))
      (return _emptyslotindex))
    (else
      (return _emptyslotindex))))

(fn FindEmptyWeaponSlot
  (LocalVariables|SetReturnIndex -1)
  (bind (_array_element _array_index) (Utilities|Array|ForEachLoopwithBreak (Variables|Default|GetRifleSlot) :!label _label)
    (:LoopBody
      (Utilities|IsValid _array_element
        (:Is%20Not%20Valid
          (LocalVariables|SetReturnIndex _array_index)
          (goto _label Break))))
    (:Completed
      (return (LocalVariables|GetReturnIndex)))))

(fn StoreRifle
  (params (OldHand :type HandType%20Enum :default "NewEnumerator0"))
  (if (Utilities|Enum|Equal(Enum) OldHand "NewEnumerator1")
    (Transformation|AttachComponentToComponent (Utilities|Array|Get(acopy) (Variables|Default|GetRifleSlot)) (Variables|Character|GetMesh) "Store Rifle Socket1" "SnapToTarget" "SnapToTarget" "KeepWorld" true)
    (Variables|Default|SetHand%20Arm "NewEnumerator0" :!label _label)
    (Variables|Default|SetHolding%20Gun? false)
    (Animation|StopAnimMontage "/Game/BluePrints/Zombie/RifleMontage.RifleMontage")
    (elif (Utilities|Enum|Equal(Enum) OldHand "NewEnumerator2")
      (Transformation|AttachComponentToComponent (Utilities|Array|Get(acopy) (Variables|Default|GetRifleSlot) 1) (Variables|Character|GetMesh) "Store Rifle Socket2" "SnapToTarget" "SnapToTarget" "KeepWorld" true)
      (goto _label))))

(fn UseRifle
  (params (WantHand :type HandType%20Enum :default "NewEnumerator0"))
  (if (Utilities|Enum|Equal(Enum) (Variables|Default|GetHand%20Arm) "NewEnumerator0")
    _
    (else
      (CallFunction|StoreRifle (Variables|Default|GetHand%20Arm))))
  (if (Utilities|Enum|Equal(Enum) WantHand "NewEnumerator1")
    (Transformation|AttachComponentToComponent (Utilities|Array|Get(acopy) (Variables|Default|GetRifleSlot)) (Variables|Character|GetMesh) "Use Rifle Socket" "SnapToTarget" "SnapToTarget" "KeepWorld" true)
    (Variables|Default|SetHand%20Arm "NewEnumerator1")
    (Variables|Default|SetHolding%20Gun? true :!label _label)
    (Animation|PlayAnimMontage "/Game/BluePrints/Zombie/RifleMontage.RifleMontage" 1.0 "None")
    (elif (Utilities|Enum|Equal(Enum) WantHand "NewEnumerator2")
      (Transformation|AttachComponentToComponent (Utilities|Array|Get(acopy) (Variables|Default|GetRifleSlot) 1) (Variables|Character|GetMesh) "Use Rifle Socket" "SnapToTarget" "SnapToTarget" "KeepWorld" true)
      (Variables|Default|SetHand%20Arm "NewEnumerator2")
      (goto _label))))

(fn Pressed1
  (Utilities|IsValid (Utilities|Array|Get(acopy) (Variables|Default|GetRifleSlot))
    (:Is%20Valid
      (if (not (or (Variables|Default|GetReloading) (Variables|Default|GetShooting?)))
        (if (Utilities|Enum|Equal(Enum) (Variables|Default|GetHand%20Arm) "NewEnumerator1")
          (CallFunction|StoreRifle (Variables|Default|GetHand%20Arm))
          (else
            (CallFunction|UseRifle "NewEnumerator1")))
        (CallFunction|UpdateUsingRifle)))))

(fn Pressed2
  (Utilities|IsValid (Utilities|Array|Get(acopy) (Variables|Default|GetRifleSlot) 1)
    (:Is%20Valid
      (if (not (or (Variables|Default|GetReloading) (Variables|Default|GetShooting?)))
        (if (Utilities|Enum|Equal(Enum) (Variables|Default|GetHand%20Arm) "NewEnumerator2")
          (CallFunction|StoreRifle (Variables|Default|GetHand%20Arm))
          (else
            (CallFunction|UseRifle "NewEnumerator2")))
        (CallFunction|UpdateUsingRifle)))))

(fn UpdateUsingRifle
  (switch Utilities|FlowControl|Switch|SwitchonHandType (Variables|Default|GetHand%20Arm)
    (:NewEnumerator0
      (Variables|Default|SetUsingRifle 0))
    (:NewEnumerator1
      (Variables|Default|SetUsingRifle (Utilities|Array|Get(acopy) (Variables|Default|GetRifleSlot))))
    (:NewEnumerator2
      (Variables|Default|SetUsingRifle (Utilities|Array|Get(acopy) (Variables|Default|GetRifleSlot) 1)))))

(fn UpdateinTick
  (Variables|Default|SetGround%20Speed (Math|Vector|VectorLengthXY (Variables|/Script/Engine.MovementComponent|GetVelocity (Variables|Character|GetCharacterMovement)))))

(fn InitialSetting
  (bind _returnvalue (Game|GetPlayerCameraManager 0))
  (Variables|/Script/Engine.PlayerCameraManager|SetViewPitchMax _returnvalue 1e+01)
  (Variables|/Script/Engine.PlayerCameraManager|SetViewPitchMin _returnvalue -15.0))