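; BP_RifleBase is a base rifle actor that can be picked up once and cleans itself up if left unclaimed.
; On BeginPlay it registers with TestGameMode's rifle-destroy event, which destroys the actor only if it has not been grabbed.
; Grab succeeds once, setting the grabbed flag and disabling actor collision, while CanPick always returns true.
; The box overlap events are empty.
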(event OnComponentBeginOverlap(Box)
  (params (OverlappedComponent :type Primitive%20Component%20Object%20Reference) (OtherActor :type Actor%20Object%20Reference) (OtherComp :type Primitive%20Component%20Object%20Reference) (OtherBodyIndex :type Integer) (bFromSweep :type Boolean) (SweepResult :type Hit%20Result%20Structure%20%28by%20ref%29)))

(event OnComponentEndOverlap(Box)
  (params (OverlappedComponent :type Primitive%20Component%20Object%20Reference) (OtherActor :type Actor%20Object%20Reference) (OtherComp :type Primitive%20Component%20Object%20Reference) (OtherBodyIndex :type Integer)))

(event Custom|Destroy%20Call
  (if (not (Variables|Default|GetGrabed?))
    (Actor|DestroyActor)))

(event EventBeginPlay
  (bind _astest_game_mode (Utilities|Casting|CastToTestGameMode (Game|GetGameMode)))
  (EventDispatchers|BindEventtoDestroyRifles _astest_game_mode (delegate Custom|Destroy%20Call)))

(event Collision|EventActorBeginOverlap
  (params (OtherActor :type Actor%20Object%20Reference)))

(event EventTick
  (params (DeltaSeconds :type Float%20%28single-precision%29)))

(fn ConstructionScript)

(fn CanPick
  (return true))

(fn Grab
  (if (Variables|Default|GetGrabed?)
    (return false)
    (else
      (Variables|Default|SetGrabed? true)
      (Collision|SetActorEnableCollision false)
      (return true))))